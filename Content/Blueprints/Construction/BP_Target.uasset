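; BP_Target is a target Blueprint that builds a grid of child actors in its construction script, sized by X and Y and spaced by Padding.
; A random bool picks one of two modulo-based patterns, leaving gaps on odd Y indices at either odd or even X indices.
; The random pick repeats whenever construction reruns, so the layout can change.
; The Hit event is an empty stub.
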(event `self.ReceiveHit`
  (params (MyComp :type "PrimitiveComponent Object Reference") (Other :type "Actor Object Reference") (OtherComp :type "PrimitiveComponent Object Reference") (bSelfMoved :type Boolean) (HitLocation :type "Vector Structure") (HitNormal :type "Vector Structure") (NormalImpulse :type "Vector Structure") (Hit :type "HitResult Structure (by ref)")))

(fn `UserConstructionScript`
  (if (`KismetMathLibrary.RandomBool`)
    (for _index (range (+ (`self.X`) 1))
      (bind _output_get (set `self.IndexX1` _index))
      (for _index_2 (range (+ (`self.Y`) 1))
        (bind _output_get_2 (set `self.IndexY1` _index_2))
        (if (or (== (mod (`self.IndexX1`) 2) 0) (== (mod (`self.IndexY1`) 2) 0))
          (`AddComponent|NODE_AddChildActorComponent-0` :`RelativeTransform` (`KismetMathLibrary.MakeTransform` (`KismetMathLibrary.MakeVector` (`KismetMathLibrary.Conv_IntToDouble` (* _output_get (`self.Padding`))) (`KismetMathLibrary.Conv_IntToDouble` (* _output_get_2 (`self.Padding`)))))))))
    (else
      (for _index_3 (range (+ (`self.X`) 1))
        (bind _output_get_3 (set `self.IndexX2` _index_3))
        (for _index_4 (range (+ (`self.Y`) 1))
          (bind _output_get_4 (set `self.IndexY2` _index_4))
          (if (or (== (mod (`self.IndexX2`) 2) 1) (!= (mod (`self.IndexY2`) 2) 1))
            (`AddComponent|NODE_AddChildActorComponent-2` :`RelativeTransform` (`KismetMathLibrary.MakeTransform` (`KismetMathLibrary.MakeVector` (`KismetMathLibrary.Conv_IntToDouble` (* _output_get_3 (`self.Padding`))) (`KismetMathLibrary.Conv_IntToDouble` (* _output_get_4 (`self.Padding`))))))))))))