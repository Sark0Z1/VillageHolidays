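; BP_Bonus is a moving bonus actor that disappears when it reaches the player's bat or a kill volume.
; Tick moves it along Direction at Speed with a swept, frame-rate-independent world offset.
; On overlap, a Sequence casts the other actor to BP_Bat and KillZVolume, destroying the bonus on either match.
; No reward is applied in this graph.
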(event `self.ReceiveActorBeginOverlap`
  (params (OtherActor :type "Actor Object Reference"))
  (`|ExecutionSequence`
    (:`then_0`
      (cast `/Game/Blueprints/Construction/BP_Bat` OtherActor)
      (`self.K2_DestroyActor`))
    (:`then_1`
      (cast `KillZVolume` OtherActor)
      (`self.K2_DestroyActor`))))

(event `self.ReceiveTick`
  (params (DeltaSeconds :type "Float (single-precision)"))
  (`self.K2_AddActorWorldOffset` (* (* (`self.direction`) (`self.speed`)) DeltaSeconds) true))

(fn `UserConstructionScript`)