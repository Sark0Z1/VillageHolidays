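; BP_Bat is the player's bat in a ball game, spawning balls and reacting to falling pickups.
; It spawns a ball at its capsule on BeginPlay and binds that ball's OnDead event to spawn and rebind a replacement.
; Overlapping BP_BBall randomly spawns either an extra ball with a cross material or a short-lived super ball.
; Overlapping BP_Lose lowers the bat's Speed, and both pickups play a sound.
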(event `self.ReceiveActorBeginOverlap`
  (params (OtherActor :type "Actor Object Reference"))
  (`|ExecutionSequence`
    (:`then_0`
      (cast `/Game/Blueprints/Construction/BP_BBall` OtherActor)
      (`GameplayStatics.PlaySoundAtLocation` "/Game/VFX/Take_a_bonus.Take_a_bonus" (`self.K2_GetActorLocation`) (struct) 1.0 1.0 0.0 null null null)
      (if (`KismetMathLibrary.RandomBool`)
        (bind _output_get (`self.SpawnBall`))
        (`PrimitiveComponent.SetMaterial` (`/Game/Blueprints/Construction/BP_Ball.StaticMesh` _output_get) 0 "/Game/Environment/Materials/M_BBall_cross.M_BBall_cross")
        (else
          (`self.SpawnSuperBall`))))
    (:`then_1`
      ;[1 1 1] Finally. If player catches negative bonus, BP_Bat will move for 20 percent slower.
      (cast `/Game/Blueprints/Construction/BP_Lose` OtherActor)
      (set `self.Speed` (- (`self.Speed`) 0.1))
      (`GameplayStatics.PlaySoundAtLocation` "/Game/VFX/Miss.Miss" (`self.K2_GetActorLocation`) (struct) 1.0 1.0 0.0 null null null))))

(event `self.ReceiveBeginPlay`
  ;[1 1 1] Spawn ball into capsule collision
  (bind _output_get (`self.SpawnBall` :!label _label))
  (add `/Game/Blueprints/Construction/BP_Ball.OnDead` _output_get (delegate `SpawnBall Event`)))

(event `SpawnBall Event`
  (goto _label))

(fn `SpawnBall`
  (returns (Output_Get :type "/Game/Blueprints/Construction/BP_Ball Object Reference"))
  (bind _returnvalue (`|SpawnActorFromClass` "/Game/Blueprints/Construction/BP_Ball.BP_Ball_C" (`KismetMathLibrary.MakeTransform` (`SceneComponent.K2_GetComponentLocation` (`self.Capsule`)) (struct) (0.75 0.75 0.75)) "AlwaysSpawn" "OverrideRootScale" null null))
  (bind _output_get (set `self.PlayingBall` _returnvalue))
  (return _output_get))

(fn `SpawnSuperBall`
  (bind _returnvalue (`|SpawnActorFromClass` "/Game/Blueprints/Construction/BP_SuperBall.BP_SuperBall_C" (`KismetMathLibrary.MakeTransform` (`SceneComponent.K2_GetComponentLocation` (`self.Capsule`)) (struct) (0.5 0.5 0.5)) "AlwaysSpawn" "OverrideRootScale" null null))
  (`self.SetLifeSpan` _returnvalue 1.0))

(fn `UserConstructionScript`)