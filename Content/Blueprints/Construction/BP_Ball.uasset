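; BP_Ball is a bouncing ball actor that travels at a set speed and direction and is lost on reaching a KillZVolume.
; Tick moves it with a swept world offset, reflecting the direction off the hit normal and playing a sound on blocking hits.
; KillZ overlap plays a sound, fires OnDead, destroys the ball, and calls EventLife on WAQ_GameMode when BallsNum is not above one.
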(event `self.ReceiveActorBeginOverlap`
  (params (OtherActor :type "Actor Object Reference"))
  ;[1 1 1] Destroy actor after hit KillZ
  (cast `KillZVolume` OtherActor)
  ;[1 1 1] Add sound effect when ball hit KillZ
  (`GameplayStatics.PlaySoundAtLocation` "/Game/VFX/zvuk2.zvuk2" (`self.K2_GetActorLocation`) (struct) 1.0 1.0 0.0 null null null)
  (`self.OnDead`)
  (`self.K2_DestroyActor`)
  (bind _aswaq_game_mode (cast `/Game/Blueprints/Game_Mechanics/WAQ_GameMode` (`GameplayStatics.GetGameMode`)))
  (if (not (> (`/Game/Blueprints/Game_Mechanics/WAQ_GameMode.BallsNum` _aswaq_game_mode) 1))
    (`/Game/Blueprints/Game_Mechanics/WAQ_GameMode.Event Life` _aswaq_game_mode (`self.Life`))))

(event `self.ReceiveTick`
  (params (DeltaSeconds :type "Float (single-precision)"))
  ;[1 1 1] We made procces, when ball has been moving on world scene with special speed and special direction. If he hit targets, he will move off to reflection direction
  (bind _sweephitresult (`self.K2_AddActorWorldOffset` (* (* (`self.Diretion`) (`self.Speed`)) DeltaSeconds) true))
  (bind (_bblockinghit _binitialoverlap _time _distance _location _impactpoint _normal) (`GameplayStatics.BreakHitResult` _sweephitresult))
  (if _bblockinghit
    (set `self.Diretion` (`KismetMathLibrary.GetReflectionVector` (`self.Diretion`) _normal))
    ;[1 1 1] Add sound effect when hit targets and dat
    (`GameplayStatics.PlaySoundAtLocation` "/Game/VFX/Hit_to_Target.Hit_to_Target" (`self.K2_GetActorLocation`) (struct) 1.0 1.0 0.0 null null null)))

(fn `UserConstructionScript`)