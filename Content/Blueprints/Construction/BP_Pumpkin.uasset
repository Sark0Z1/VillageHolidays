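; BP_Pumpkin is a breakable target that takes two ball hits to destroy and adds to the game score.
; The first hit swaps the mesh material to Seam; the next calls CallCrushPump, destroys the actor and passes Total to WAQ_GameMode's TotalScore.
; A random roll against Random then decides whether a bonus spawns at its location, with a second even roll choosing BP_BBall or BP_Lose.
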(event `self.ReceiveHit`
  (params (MyComp :type "PrimitiveComponent Object Reference") (Other :type "Actor Object Reference") (OtherComp :type "PrimitiveComponent Object Reference") (bSelfMoved :type Boolean) (HitLocation :type "Vector Structure") (HitNormal :type "Vector Structure") (NormalImpulse :type "Vector Structure") (Hit :type "HitResult Structure (by ref)"))
  ;[1 1 1] This logical tell us, how many pumpkins will make at BP_Target. Then we know, if we hit him first time actor change his material. But when ball hit him second time, he will destroy
  (set `self.Hits` (+ (`self.Hits`) 1))
  (if (== (`self.Hits`) 1)
    (`PrimitiveComponent.SetMaterial` (`self.StaticMesh`) 0 "/Game/Environment/Meshes/seam.seam")
    (else
      (`self.CrushPump`)
      (`self.K2_DestroyActor`)
      ;[1 1 1] Pumpkins will be counted after destroy
      (bind _aswaq_game_mode (cast `/Game/Blueprints/Game_Mechanics/WAQ_GameMode` (`GameplayStatics.GetGameMode`)))
      (`/Game/Blueprints/Game_Mechanics/WAQ_GameMode.TotalScore` _aswaq_game_mode (`self.Total`))
      ;[1 1 1] After destroy we need spawn some bonus. Will be great, if there bonus create at random
      (if (< (`KismetMathLibrary.RandomFloat`) (`self.Random`))
        ;[1 1 1] And here we get to know, positive or negative bonus we have. Of course it will random
        (if (< (`KismetMathLibrary.RandomFloatInRange` 0.1 0.2) 0.15)
          (`|SpawnActorFromClass` "/Game/Blueprints/Construction/BP_BBall.BP_BBall_C" (`KismetMathLibrary.MakeTransform` (`self.K2_GetActorLocation`)) "AlwaysSpawn" "OverrideRootScale" null null)
          (else
            (`|SpawnActorFromClass` "/Game/Blueprints/Construction/BP_Lose.BP_Lose_C" (`KismetMathLibrary.MakeTransform` (`self.K2_GetActorLocation`)) "AlwaysSpawn" "OverrideRootScale" null null)))))))

(fn `UserConstructionScript`)