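; Game mode for a top-down ball-and-pumpkin game, tracking score, lives and game over.
; BeginPlay spawns a downward-facing camera as the view target and plays the game music.
; TotalScore accumulates points against BP_Target's pumpkin count, obtained by casting its own owner, while Life subtracts lives; either limit shows the same game-over widget and pauses.
; Tick refreshes the list and count of BP_Ball actors.
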(event `self.ReceiveBeginPlay`
  ;[1 1 1] Create a camera
  (bind _returnvalue (`|SpawnActorFromClass` "/Script/Engine.CameraActor" (`KismetMathLibrary.MakeTransform` (`self.height`) (struct :`Pitch` -90.0)) "Undefined" "OverrideRootScale" null null))
  (`PlayerController.SetViewTargetWithBlend` (`GameplayStatics.GetPlayerController` 0) _returnvalue 0.0 "VTBlend_Linear" 0.0 false)
  ;[1 1 1] We add game sound with loop
  (`GameplayStatics.PlaySoundAtLocation` "/Game/VFX/Music_Game.Music_Game" (0.0 0.0 0.0) (struct) 1.0 1.0 0.0 null null null))

(event `TotalScore`
  (params (Value :type Integer :default 1))
  (bind _returnvalue (`GameplayStatics.GetPlayerController` 0))
  ;[1 1 1] Add Event where we made Total variables
  (set `self.Total` (+ Value (`self.Total`)))
  (bind _asbp_target (cast `/Game/Blueprints/Construction/BP_Target` (`self.GetOwner`)))
  (if (== (`self.Total`) (`/Game/Blueprints/Construction/BP_Target.TotalPumpkinsOnMap` _asbp_target))
    (bind _returnvalue_2 (`|CreateWidget` "/Game/HUD/GameOver/GameOver_WidgetBP.GameOver_WidgetBP_C"))
    (`UserWidget.AddToViewport` _returnvalue_2 0)
    (set `PlayerController.bShowMouseCursor` true _returnvalue)
    (`GameplayStatics.SetGamePaused` true)
    (`WidgetBlueprintLibrary.SetInputMode_GameAndUIEx` _returnvalue _returnvalue_2)))

(event `Event Life`
  (params (Value :type Integer))
  (bind _returnvalue (`GameplayStatics.GetPlayerController` 0))
  (set `self.Life` (- (`self.Life`) Value))
  (if (< (`self.Life`) 1)
    (bind _returnvalue_2 (`|CreateWidget` "/Game/HUD/GameOver/GameOver_WidgetBP.GameOver_WidgetBP_C"))
    (`UserWidget.AddToViewport` _returnvalue_2 0)
    (set `PlayerController.bShowMouseCursor` true _returnvalue)
    (`GameplayStatics.SetGamePaused` true)
    (`WidgetBlueprintLibrary.SetInputMode_GameAndUIEx` _returnvalue _returnvalue_2)))

(event `self.ReceiveTick`
  (params (DeltaSeconds :type "Float (single-precision)"))
  (bind _outactors (`GameplayStatics.GetAllActorsOfClass` "/Game/Blueprints/Construction/BP_Ball.BP_Ball_C"))
  (bind _output_get (set `self.Balls` _outactors))
  (set `self.BallsNum` (`KismetArrayLibrary.Array_Length` _output_get)))

(fn `UserConstructionScript`)